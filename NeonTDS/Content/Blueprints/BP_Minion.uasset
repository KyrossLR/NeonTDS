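; BP_Minion is a minion actor that sets up its own look, with a black metallic body and a glowing red eye.
; BeginPlay calls Initialize, which runs SetColors to create dynamic material instances from metallic and emissive parent materials and apply them to the Body and Eye components.
; Update is an empty stub, and the construction script only calls its parent, so the colors are applied at runtime.
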(event `self.ReceiveBeginPlay`
  (`self.Initialize`))

(fn `Initialize`
  (`self.SetColors`))

(fn `SetColors`
  ;[1 1 1] Set Body Color
  (bind _returnvalue (`KismetMaterialLibrary.CreateDynamicMaterialInstance` "/Game/Materials/M_MetallicSolid.M_MetallicSolid"))
  (`MaterialInstanceDynamic.SetVectorParameterValue` _returnvalue "BaseColor" (make `LinearColor` 0.0 0.0 0.0 1.0))
  (`PrimitiveComponent.SetMaterial` (`self.Body`) 0 _returnvalue)
  ;[1 1 1] Set Eye Color
  (bind _returnvalue_2 (`KismetMaterialLibrary.CreateDynamicMaterialInstance` "/Game/Materials/M_EmissiveSolid.M_EmissiveSolid"))
  (`MaterialInstanceDynamic.SetVectorParameterValue` _returnvalue_2 "EmissiveColor" (make `LinearColor` 1.0 0.0 0.0 1.0))
  (`PrimitiveComponent.SetMaterial` (`self.Eye`) 0 _returnvalue_2))

(fn `Update`)

(fn `UserConstructionScript`
  (`parent.UserConstructionScript`))