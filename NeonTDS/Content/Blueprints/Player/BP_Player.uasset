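; Player pawn for a top-down shooter that moves on world axes, faces the mouse cursor and fires BP_Bullet from ShootingSource with a delay-gated cooldown.
; Tick applies swept movement scaled by SpeedMax over frame delta, and aims by deprojecting the cursor at camera-to-body distance.
; Damage lowers Health and blends the health ball's dynamic material color.
; At zero health, Tick repeatedly calls OnDeath, which hides the player and reloads Map_Default after a delay.
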(event `self.ReceiveBeginPlay`
  ;[1 1 1] Initialize
  (`self.Initialize`))

(event `self.ReceiveTick`
  (params (DeltaSeconds :type "Float (single-precision)"))
  ;[1 1 1] Update
  (bind _isdead (`self.IsDead`))
  (if _isdead
    (`self.OnDeath`)
    (else
      (`self.Update`))))

(event `InputAxis|Move_Forward`
  (params (AxisValue :type "Float (single-precision)"))
  ;[1 1 1] Get Movement Inputs
  (`self.AddMovementInput` (1.0 0.0 0.0) AxisValue))

(event `InputAxis|Shoot_Bullet`
  (params (AxisValue :type "Float (single-precision)"))
  (bind (_returnvalue_location _returnvalue_rotation) (`KismetMathLibrary.BreakTransform` (`SceneComponent.K2_GetComponentToWorld` (`self.ShootingSource`))))
  (bind _isdead (`self.IsDead`))
  (if (and (not _isdead) (> AxisValue 0.0) (`self.CanShoot`))
    (`|SpawnActorFromClass` "/Game/Blueprints/Weapons/BP_Bullet.BP_Bullet_C" (`KismetMathLibrary.MakeTransform` _returnvalue_location _returnvalue_rotation) "Undefined" "OverrideRootScale" null null)
    (set `self.CanShoot` false)
    (`KismetSystemLibrary.Delay` (`self.ShootDelay_Bullet`))
    (set `self.CanShoot` true)))

(event `InputAxis|Move_Right`
  (params (AxisValue :type "Float (single-precision)"))
  ;[1 1 1] Get Movement Inputs
  (`self.AddMovementInput` (0.0 1.0 0.0) AxisValue))

(event `self.ReceiveAnyDamage`
  (params (Damage :type "Float (single-precision)") (DamageType :type "DamageType Object Reference") (InstigatedBy :type "Controller Object Reference") (DamageCauser :type "Actor Object Reference"))
  ;[1 1 1] Receive Damage
  (`self.TakeDamage` Damage))

(event `OnDeath`
  ;[1 1 1] Die
  (`SceneComponent.SetVisibility` (`self.CollisionBox`) false true)
  (`KismetSystemLibrary.Delay` 3.0)
  (`GameplayStatics.OpenLevel` "Map_Default"))

(fn `FaceCursor`
  (bind _returnvalue (`self.K2_GetActorLocation`))
  (bind (_worldlocation _worlddirection) (`PlayerController.DeprojectMousePositionToWorld` (`GameplayStatics.GetPlayerController` 0)))
  (`self.K2_SetActorRotation` (`KismetMathLibrary.FindLookAtRotation` _returnvalue (`KismetMathLibrary.MakeVector` (.x (+ _worldlocation (* _worlddirection (`KismetMathLibrary.VSize` (- (`SceneComponent.K2_GetComponentLocation` (`self.Body`)) (`SceneComponent.K2_GetComponentLocation` (`self.Camera`))))))) (.y (+ _worldlocation (* _worlddirection (`KismetMathLibrary.VSize` (- (`SceneComponent.K2_GetComponentLocation` (`self.Body`)) (`SceneComponent.K2_GetComponentLocation` (`self.Camera`))))))) (.z _returnvalue)))))

(fn `Initialize`
  (`self.SetVariablesToDefault`)
  (`self.SetColors`)
  (`GameplayStatics.SpawnEmitterAtLocation` "/Game/ParticleSystems/PS_PlayerWarp.PS_PlayerWarp" (`self.K2_GetActorLocation`))
  (`GameplayStatics.SpawnEmitterAttached` "/Game/ParticleSystems/PS_PlayerTrail.PS_PlayerTrail" (`self.Body`) "None" (0.0 0.0 0.0) (struct) (1.0 1.0 10.0)))

(fn `IsDead`
  (returns (IsDead :type Boolean))
  (return (<= (`self.Health`) 0.0)))

(fn `Move`
  (bind _returnvalue (`self.ConsumeMovementInputVector`))
  (`self.K2_AddActorWorldOffset` (* _returnvalue (* (`self.Speed_Max`) (/ 1.0 (`GameplayStatics.GetWorldDeltaSeconds`)))) true))

(fn `SetColors`
  ;[1 1 1] Set Body Color
  (bind _returnvalue (`KismetMaterialLibrary.CreateDynamicMaterialInstance` "/Game/Materials/M_MetallicSolid.M_MetallicSolid"))
  (`MaterialInstanceDynamic.SetVectorParameterValue` _returnvalue "BaseColor" (make `LinearColor` 0.0 0.0 0.0 1.0))
  (`PrimitiveComponent.SetMaterial` (`self.Body`) 0 _returnvalue)
  ;[1 1 1] Set Eye Color
  (bind _returnvalue_2 (`KismetMaterialLibrary.CreateDynamicMaterialInstance` "/Game/Materials/M_EmissiveSolid.M_EmissiveSolid"))
  (`MaterialInstanceDynamic.SetVectorParameterValue` _returnvalue_2 "EmissiveColor" (make `LinearColor` 0.0 0.0 1.0 1.0))
  (`PrimitiveComponent.SetMaterial` (`self.Eye`) 0 _returnvalue_2)
  ;[1 1 1] Set Health Ball Color
  (bind _returnvalue_3 (`KismetMaterialLibrary.CreateDynamicMaterialInstance` "/Game/Materials/M_EmissiveSolid.M_EmissiveSolid"))
  (bind _output_get (set `self.HealthBall_Material` _returnvalue_3))
  (`PrimitiveComponent.SetMaterial` (`self.HealthBall`) 0 _output_get)
  (`self.UpdateHealthBallColor`))

(fn `SetVariablesToDefault`
  (set `self.Health` (`self.Health_Max`))
  (set `self.CanShoot` true))

(fn `TakeDamage`
  (params (Damage :type "Float (double-precision)"))
  (set `self.Health` (- (`self.Health`) Damage))
  (`self.UpdateHealthBallColor`))

(fn `Update`
  (`self.Move`)
  (`self.FaceCursor`))

(fn `UpdateHealthBallColor`
  (`MaterialInstanceDynamic.SetVectorParameterValue` (`self.HealthBall_Material`) "EmissiveColor" (`KismetMathLibrary.LinearColorLerp` (`self.HealthBall_DeathColor`) (`self.HealthBall_FullColor`) (/ (`self.Health`) (`self.Health_Max`)))))

(fn `UserConstructionScript`
  (`parent.UserConstructionScript`))