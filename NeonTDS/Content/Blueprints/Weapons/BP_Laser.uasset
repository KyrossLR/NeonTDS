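; BP_Laser is a laser projectile that damages characters and can be turned into a homing shot.
; Overlapping a Character applies its Damage, spawns a small explosion and destroys the laser; hitting a BlockingVolume explodes and destroys it without damage.
; The HomingLaser event points the projectile movement at a target's capsule with very high homing acceleration and attaches a trail effect to the laser.
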(event `self.ReceiveActorBeginOverlap`
  (params (OtherActor :type "Actor Object Reference"))
  (bind _ascharacter (cast `Character` OtherActor)
    (:`then`
      (`GameplayStatics.ApplyDamage` _ascharacter (`self.Damage`)))
    (:`CastFailed`
      (cast `BlockingVolume` OtherActor)))
  (`GameplayStatics.SpawnEmitterAtLocation` "/Game/ParticleSystems/PS_PlayerExplosion.PS_PlayerExplosion" (`self.K2_GetActorLocation` self) (struct) (0.2 0.2 0.2))
  (`self.K2_DestroyActor`))

(event `HomingLaser`
  (params (HomingTarget :type "/Game/Blueprints/Enemies/BP_EnemyClass Object Reference"))
  (bind _projectilemovement (`self.ProjectileMovement`))
  (if (`KismetSystemLibrary.IsValid` HomingTarget)
    (set `ProjectileMovementComponent.HomingTargetComponent` (`Character.CapsuleComponent` HomingTarget) _projectilemovement)
    (set `ProjectileMovementComponent.bIsHomingProjectile` true _projectilemovement)
    (set `ProjectileMovementComponent.HomingAccelerationMagnitude` 200000.0 _projectilemovement)
    (`GameplayStatics.SpawnEmitterAttached` "/Game/ParticleSystems/PS_PlayerTrail.PS_PlayerTrail" (`self.Laser`) "None" (0.0 0.0 0.0) (struct) (2.0 2.0 2.0))))

(fn `UserConstructionScript`)