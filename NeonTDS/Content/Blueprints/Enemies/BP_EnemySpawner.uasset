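; BP_EnemySpawner is an enemy spawner that periodically spawns BP_Minion actors within a box area.
; Tick counts a timer down, spawns a minion at the FindSpawnLocation result, then resets the timer.
; FindSpawnLocation samples random X and Y inside SpawningArea at the player's height, looping while Distance is below MinDistanceToPlayer from the BP_Player cached on BeginPlay.
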(event `self.ReceiveBeginPlay`
  (bind _asbp_player (cast `/Game/Blueprints/Player/BP_Player` (`GameplayStatics.GetPlayerPawn` 0)))
  (set `self.Player` _asbp_player))

(event `self.ReceiveTick`
  (params (DeltaSeconds :type "Float (single-precision)"))
  (bind _output_get (set `self.tmpTimer` (- (`self.tmpTimer`) DeltaSeconds)))
  (if (<= _output_get 0.0)
    (bind _spawnlocation (`self.FindSpawnLocation`))
    (`|SpawnActorFromClass` "/Game/Blueprints/Enemies/Minion/BP_Minion.BP_Minion_C" (`KismetMathLibrary.MakeTransform` _spawnlocation) "Undefined" "OverrideRootScale" null null)
    (set `self.tmpTimer` (`self.tmpTimer_Max`))))

(fn `FindSpawnLocation`
  (returns (SpawnLocation :type "Vector Structure"))
  (locals (Distance :type "Float (double-precision)" :default 0.0) (Location :type "Vector Structure"))
  (bind _spawningarea (`self.SpawningArea`))
  (bind (_returnvalue_x _returnvalue_y _returnvalue_z) (`KismetMathLibrary.BreakVector` (`self.K2_GetActorLocation` (`self.Player`))))
  (bind (_returnvalue_x_2 _returnvalue_y_2) (`KismetMathLibrary.BreakVector` (`KismetMathLibrary.RandomPointInBoundingBox` (`SceneComponent.K2_GetComponentLocation` _spawningarea) (`BoxComponent.BoxExtent` _spawningarea))))
  (while (< (`local.Distance`) (`self.MinDistanceToPlayer`))
    (bind _output_get (set `local.Location` (`KismetMathLibrary.MakeVector` _returnvalue_x_2 _returnvalue_y_2 _returnvalue_z)))
    (set `local.Distance` (`KismetMathLibrary.VSize` (- (`self.K2_GetActorLocation` (`self.Player`)) _output_get))))
  (return (`local.Location`)))

(fn `UserConstructionScript`)