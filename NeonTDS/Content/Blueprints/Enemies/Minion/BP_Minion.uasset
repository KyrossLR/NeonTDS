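; Minion enemy character that damages the player on contact and destroys itself in the process.
; On BeginPlay, it builds dynamic materials for a black body and glowing red eye, applies its top walk speed and spawns a warp particle effect.
; A capsule overlap with a living BP_Player applies contact damage, then calls OnDeath, which destroys the actor.
; The Update function is an empty stub, and no movement logic lives here.
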(event `self.ReceiveBeginPlay`
  (`self.Initialize`))

(event `self.CapsuleComponent.OnComponentBeginOverlap`
  (params (OverlappedComponent :type "PrimitiveComponent Object Reference") (OtherActor :type "Actor Object Reference") (OtherComp :type "PrimitiveComponent Object Reference") (OtherBodyIndex :type Integer) (bFromSweep :type Boolean) (SweepResult :type "HitResult Structure (by ref)"))
  (bind _asbp_player (cast `/Game/Blueprints/Player/BP_Player` OtherActor))
  (bind _isdead (`/Game/Blueprints/Player/BP_Player.IsDead` _asbp_player))
  (if (not _isdead)
    (`GameplayStatics.ApplyDamage` _asbp_player (`self.DamageOnContact`))
    (`self.OnDeath`)))

(event `OnDeath`
  (`self.K2_DestroyActor`))

(fn `Initialize`
  (`self.SetColors`)
  (set `CharacterMovementComponent.MaxWalkSpeed` (`self.Speed_Max`) (`self.CharacterMovement`))
  (`GameplayStatics.SpawnEmitterAtLocation` "/Game/ParticleSystems/PS_Warp.PS_Warp" (`self.K2_GetActorLocation`)))

(fn `SetColors`
  ;[1 1 1] Set Body Color
  (bind _returnvalue (`KismetMaterialLibrary.CreateDynamicMaterialInstance` "/Game/Materials/M_MetallicSolid.M_MetallicSolid"))
  (`MaterialInstanceDynamic.SetVectorParameterValue` _returnvalue "BaseColor" (make `LinearColor` 0.0 0.0 0.0 1.0))
  (`PrimitiveComponent.SetMaterial` (`self.Body`) 0 _returnvalue)
  ;[1 1 1] Set Eye Color
  (bind _returnvalue_2 (`KismetMaterialLibrary.CreateDynamicMaterialInstance` "/Game/Materials/M_EmissiveSolid.M_EmissiveSolid"))
  (`MaterialInstanceDynamic.SetVectorParameterValue` _returnvalue_2 "EmissiveColor" (make `LinearColor` 1.0 0.0 0.0 1.0))
  (`PrimitiveComponent.SetMaterial` (`self.Eye`) 0 _returnvalue_2))

(fn `Update`)

(fn `UserConstructionScript`
  (`parent.UserConstructionScript`))