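; Player actor that moves along world X/Y axes and turns to face the mouse cursor.
; BeginPlay applies dynamic materials for a black body and emissive blue eye.
; Each Tick consumes accumulated movement input as a swept world offset, scaled by SpeedMax divided by delta time.
; Facing deprojects the cursor to the camera-to-body distance, then looks at that point at the actor's own height.
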(event `self.ReceiveBeginPlay`
  (`self.Initialize`))

(event `InputAxis|Move_Forward`
  (params (AxisValue :type "Float (single-precision)"))
  ;[1 1 1] Get Movement Inputs
  (`self.AddMovementInput` (1.0 0.0 0.0) AxisValue))

(event `InputAxis|Move_Right`
  (params (AxisValue :type "Float (single-precision)"))
  ;[1 1 1] Get Movement Inputs
  (`self.AddMovementInput` (0.0 1.0 0.0) AxisValue))

(event `self.ReceiveTick`
  (params (DeltaSeconds :type "Float (single-precision)"))
  (`self.Update`))

(fn `FaceCursor`
  (bind _returnvalue (`self.K2_GetActorLocation`))
  (bind (_worldlocation _worlddirection) (`PlayerController.DeprojectMousePositionToWorld` (`GameplayStatics.GetPlayerController` 0)))
  (`self.K2_SetActorRotation` (`KismetMathLibrary.FindLookAtRotation` _returnvalue (`KismetMathLibrary.MakeVector` (.x (+ _worldlocation (* _worlddirection (`KismetMathLibrary.VSize` (- (`SceneComponent.K2_GetComponentLocation` (`self.Body`)) (`SceneComponent.K2_GetComponentLocation` (`self.Camera`))))))) (.y (+ _worldlocation (* _worlddirection (`KismetMathLibrary.VSize` (- (`SceneComponent.K2_GetComponentLocation` (`self.Body`)) (`SceneComponent.K2_GetComponentLocation` (`self.Camera`))))))) (.z _returnvalue)))))

(fn `Initialize`
  (`self.SetColors`))

(fn `Move`
  (bind _returnvalue (`self.ConsumeMovementInputVector`))
  (`self.K2_AddActorWorldOffset` (* _returnvalue (* (`self.Speed_Max`) (/ 1.0 (`GameplayStatics.GetWorldDeltaSeconds`)))) true))

(fn `SetColors`
  ;[1 1 1] Set Body Color
  (bind _returnvalue (`KismetMaterialLibrary.CreateDynamicMaterialInstance` "/Game/Materials/M_MetallicSolid.M_MetallicSolid"))
  (`MaterialInstanceDynamic.SetVectorParameterValue` _returnvalue "BaseColor" (make `LinearColor` 0.0 0.0 0.0 1.0))
  (`PrimitiveComponent.SetMaterial` (`self.Body`) 0 _returnvalue)
  ;[1 1 1] Set Eye Color
  (bind _returnvalue_2 (`KismetMaterialLibrary.CreateDynamicMaterialInstance` "/Game/Materials/M_EmissiveSolid.M_EmissiveSolid"))
  (`MaterialInstanceDynamic.SetVectorParameterValue` _returnvalue_2 "EmissiveColor" (make `LinearColor` 0.0 0.0 1.0 1.0))
  (`PrimitiveComponent.SetMaterial` (`self.Eye`) 0 _returnvalue_2))

(fn `Update`
  (`self.Move`)
  (`self.FaceCursor`))

(fn `UserConstructionScript`
  (`parent.UserConstructionScript`))